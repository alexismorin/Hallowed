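; Enemy ghost that chases the player pawn and kills it on close contact.
; A looping timer reissues AIMoveTo toward the player, while Tick feeds the anim Blueprint and checks kill distance.
; While off-screen, a second timer moves it to the spawnable BP_GhostTeleportPoint nearest the player, outside a minimum radius, with a beat sound.
; Coming into view plays a sighting sound, throttled by a delayed DoOnce reset.
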(event `BeatMaker`
  (if (`self.WasRecentlyRendered` 0.2)
    (if (not (`self.visible`))
      (set `self.visible` true)
      (`/Engine/EditorBlueprintResources/StandardMacros.DoOnce` false :!label _label
        (:`Completed`
          (`GameplayStatics.PlaySound2D` "/Game/Audio/SFX/SeeGhost.SeeGhost" 1.0 1.0 0.0 null null)
          (`KismetSystemLibrary.Delay` 5.0)
          (goto _label :!via `Reset`))))
    (else
      (set `self.visible` false))))

(event `KillPlayer`
  (`/Engine/EditorBlueprintResources/StandardMacros.DoOnce` false
    (:`Completed`
      (`/Game/Blueprints/BP_Protag.Die` (`self.target`) (+ (`self.K2_GetActorLocation`) (0.0 0.0 75.0))))))

(event `self.ReceiveTick`
  (params (DeltaSeconds :type "Float (single-precision)"))
  (`self.BeatMaker`)
  (set `/Game/Characters/Ghost/ABP_Ghost.velocity` (/ (`CharacterMovementComponent.MaxWalkSpeed` (`self.CharacterMovement`)) (`KismetMathLibrary.VSizeXY` (`CharacterMovementComponent.GetLastUpdateVelocity` (`self.CharacterMovement`)))) (`self.animBP`))
  (if (< (`self.GetDistanceTo` (`self.target`)) 50.0)
    (`self.KillPlayer`)))

(event `self.ReceiveBeginPlay`
  (`self.setupTeleports`)
  (bind _asbp_protag (cast `/Game/Blueprints/BP_Protag` (`GameplayStatics.GetPlayerPawn` 0)))
  (set `self.target` _asbp_protag)
  (bind _asabp_ghost (cast `/Game/Characters/Ghost/ABP_Ghost` (`SkeletalMeshComponent.GetAnimInstance` (`self.Mesh`))))
  (set `self.animBP` _asabp_ghost)
  (`KismetSystemLibrary.K2_SetTimerDelegate` (delegate `AIStep`) 0.2 true)
  (`KismetSystemLibrary.K2_SetTimerDelegate` (delegate `Teleport`) 1.0 true))

(event `Teleport`
  (set `self.teleportPoint` null)
  (set `self.closestTeleportPoint` 100000.0)
  (if (not (`self.WasRecentlyRendered` 0.0))
    (for _array_element (`self.teleportPoints`)
      (`/Game/Blueprints/LevelDesign/BP_GhostTeleportPoint.CheckRender` _array_element))
    (for _array_element_2 (`self.teleportPoints`)
      (bind _returnvalue (`self.GetDistanceTo` (`self.target`) _array_element_2))
      (if (< _returnvalue (`self.closestTeleportPoint`))
        (if (> _returnvalue 200.0)
          (if (`/Game/Blueprints/LevelDesign/BP_GhostTeleportPoint.canSpawn` _array_element_2)
            (set `self.teleportPoint` _array_element_2)
            (set `self.closestTeleportPoint` _returnvalue)))))
    (if (`KismetSystemLibrary.IsValid` (`self.teleportPoint`))
      (`self.K2_SetActorLocation` (+ (`self.K2_GetActorLocation` (`self.teleportPoint`)) (0.0 0.0 100.0)))
      (`GameplayStatics.PlaySound2D` "/Game/Audio/SFX/Beat.Beat" 1.0 1.0 0.0 null null))))

(event `AIStep`
  (`|AIMoveTo` (`PawnMovementComponent.GetPawnOwner` (`self.CharacterMovement`)) (`self.K2_GetActorLocation` (`self.target`)) null))

(event `setupTeleports`
  (bind _outactors (`GameplayStatics.GetAllActorsOfClass` "/Game/Blueprints/LevelDesign/BP_GhostTeleportPoint.BP_GhostTeleportPoint_C"))
  (set `self.teleportPoints` _outactors))

(fn `UserConstructionScript`)