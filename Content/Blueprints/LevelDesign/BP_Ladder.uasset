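; BP_Ladder is a ladder actor that moves BP_Protag between bottom and top snap points.
; Top and bottom trigger overlaps store the player and travel direction, then either register it as an interactable or fire immediately.
; Interact, also called on any damage, runs TriggerEvent, optionally only once.
; TriggerEvent calls SnapPawnToLocation on the player for each end in order, with fixed delays, then calls EndLock.
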(event `self.ReceiveAnyDamage`
  (params (Damage :type "Float (single-precision)") (DamageType :type "DamageType Object Reference") (InstigatedBy :type "Controller Object Reference") (DamageCauser :type "Actor Object Reference"))
  (`self.Interact`))

(event `self.ReceiveActorEndOverlap`
  (params (OtherActor :type "Actor Object Reference"))
  (bind _asbp_protag (cast `/Game/Blueprints/BP_Protag` OtherActor))
  (if (`self.interactable`)
    (`/Game/Blueprints/BP_Protag.ExitInteractable` _asbp_protag)))

(event `self.upTrigger.OnComponentBeginOverlap`
  (params (OverlappedComponent :type "PrimitiveComponent Object Reference") (OtherActor :type "Actor Object Reference") (OtherComp :type "PrimitiveComponent Object Reference") (OtherBodyIndex :type Integer) (bFromSweep :type Boolean) (SweepResult :type "HitResult Structure (by ref)"))
  (bind _asbp_protag (cast `/Game/Blueprints/BP_Protag` OtherActor))
  (set `self.player` _asbp_protag)
  (set `self.goingDown` false)
  (if (`self.interactable`) :!label _label
    (`/Game/Blueprints/BP_Protag.EnterInteractable` (`self.player`) self)
    (else
      (if (`self.doOnce`) :!label _label_2
        (`/Engine/EditorBlueprintResources/StandardMacros.DoOnce` false
          (:`Completed`
            (`self.TriggerEvent`)))
        (else
          (`self.TriggerEvent`))))))

(event `self.downTrigger.OnComponentBeginOverlap`
  (params (OverlappedComponent :type "PrimitiveComponent Object Reference") (OtherActor :type "Actor Object Reference") (OtherComp :type "PrimitiveComponent Object Reference") (OtherBodyIndex :type Integer) (bFromSweep :type Boolean) (SweepResult :type "HitResult Structure (by ref)"))
  (bind _asbp_protag (cast `/Game/Blueprints/BP_Protag` OtherActor))
  (set `self.player` _asbp_protag)
  (set `self.goingDown` true)
  (goto _label))

(event `Interact`
  (goto _label_2))

(event `TriggerEvent`
  (bind _topsnap (`self.topSnap`))
  (bind _bottomsnap (`self.bottomSnap`))
  (bind _topsnap_2 (`self.topSnap`))
  (bind _bottomsnap_2 (`self.bottomSnap`))
  (if (`self.goingDown`)
    (`/Game/Blueprints/BP_Protag.SnapPawnToLocation` (`self.player`) (`SceneComponent.K2_GetComponentLocation` _topsnap) (`SceneComponent.K2_GetComponentRotation` _topsnap))
    (`KismetSystemLibrary.Delay` 1.0)
    (`/Game/Blueprints/BP_Protag.SnapPawnToLocation` (`self.player`) (`SceneComponent.K2_GetComponentLocation` _bottomsnap_2) (`SceneComponent.K2_GetComponentRotation` _bottomsnap_2))
    (`KismetSystemLibrary.Delay` 1.0)
    (`/Game/Blueprints/BP_Protag.EndLock` (`self.player`))
    (else
      (`/Game/Blueprints/BP_Protag.SnapPawnToLocation` (`self.player`) (`SceneComponent.K2_GetComponentLocation` _bottomsnap) (`SceneComponent.K2_GetComponentRotation` _bottomsnap))
      (`KismetSystemLibrary.Delay` 1.0)
      (`/Game/Blueprints/BP_Protag.SnapPawnToLocation` (`self.player`) (`SceneComponent.K2_GetComponentLocation` _topsnap_2) (`SceneComponent.K2_GetComponentRotation` _topsnap_2))
      (`KismetSystemLibrary.Delay` 1.0)
      (`/Game/Blueprints/BP_Protag.EndLock` (`self.player`)))))

(fn `UserConstructionScript`)