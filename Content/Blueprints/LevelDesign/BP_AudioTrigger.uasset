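; BP_AudioTrigger is a level design trigger that plays gameplay audio and shows subtitles when the player enters it.
; On overlap it casts to BP_Protag and stores it, optionally passing through a DoOnce gate based on a flag.
; TriggerEvent then has the player play the Audio if valid and display DisplayText as subtitles.
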(event `self.ReceiveActorBeginOverlap`
  (params (OtherActor :type "Actor Object Reference"))
  (bind _asbp_protag (cast `/Game/Blueprints/BP_Protag` OtherActor))
  (set `self.player` _asbp_protag)
  (if (`self.doOnce`)
    (`/Engine/EditorBlueprintResources/StandardMacros.DoOnce` false
      (:`Completed`
        (`self.TriggerEvent`)))
    (else
      (`self.TriggerEvent`))))

(event `TriggerEvent`
  (bind _player (`self.player`))
  (if (`KismetSystemLibrary.IsValid` (`self.audio`))
    (`/Game/Blueprints/BP_Protag.gameplayAudioPlayback` _player (`self.audio`)))
  (`/Game/Blueprints/BP_Protag.DisplaySubtitles` _player (`self.displayText`)))

(fn `UserConstructionScript`)