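; BP_Door is a physics-constrained door that swings open when hit and snaps shut on interaction or any damage.
; It registers itself as the player's interactable while BP_Protag overlaps it.
; The first hit on a closed door plays the open sound and runs a timeline on angular damping.
; Closing plays a sound, zeroes angular velocity while a timeline drives the swing limit, then restores that limit and clears Opened.
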(event `self.ReceiveAnyDamage`
  (params (Damage :type "Float (single-precision)") (DamageType :type "DamageType Object Reference") (InstigatedBy :type "Controller Object Reference") (DamageCauser :type "Actor Object Reference"))
  (`self.Interact`))

(event `self.ReceiveActorEndOverlap`
  (params (OtherActor :type "Actor Object Reference"))
  (bind _asbp_protag (cast `/Game/Blueprints/BP_Protag` OtherActor))
  (`/Game/Blueprints/BP_Protag.ExitInteractable` _asbp_protag))

(event `self.ReceiveActorBeginOverlap`
  (params (OtherActor :type "Actor Object Reference"))
  (bind _asbp_protag (cast `/Game/Blueprints/BP_Protag` OtherActor))
  (set `self.player` _asbp_protag)
  (`/Game/Blueprints/BP_Protag.EnterInteractable` (`self.player`) self))

(event `Interact`
  (bind _physicsconstraint (`self.PhysicsConstraint`))
  (bind _door (`self.Door`))
  (`AudioComponent.SetSound` (`self.Audio`) "/Game/Audio/SFX/Door_Close.Door_Close")
  (`AudioComponent.Play` (`self.Audio`) 0.0)
  (bind (_direction _spline) (`Timeline|TL_SnapDoor` :!via `PlayFromStart`)
    (:`Update`
      (`PrimitiveComponent.SetPhysicsAngularVelocityInDegrees` _door (0.0 0.0 0.0) false "None")
      (`PhysicsConstraintComponent.SetAngularSwing1Limit` _physicsconstraint "ACM_Limited" _spline))
    (:`Finished`
      (`PrimitiveComponent.SetPhysicsAngularVelocityInDegrees` _door (0.0 0.0 0.0) false "None")
      (`PhysicsConstraintComponent.SetAngularSwing1Limit` _physicsconstraint "ACM_Limited" 90.0)
      (set `self.opened` false))))

(event `self.Door.OnComponentHit`
  (params (HitComponent :type "PrimitiveComponent Object Reference") (OtherActor :type "Actor Object Reference") (OtherComp :type "PrimitiveComponent Object Reference") (NormalImpulse :type "Vector Structure") (Hit :type "HitResult Structure (by ref)"))
  (bind _audio (`self.Audio`))
  (if (not (`self.opened`))
    (`AudioComponent.SetSound` _audio "/Game/Audio/SFX/Door_Open.Door_Open")
    (`AudioComponent.Play` _audio 0.0)
    (set `self.opened` true)
    (bind (_direction _newtrack_0) (`Timeline|TL_ReleaseTension` :!via `PlayFromStart`)
      (:`Update`
        (`PrimitiveComponent.SetAngularDamping` (`self.Door`) _newtrack_0)))))

(fn `UserConstructionScript`)