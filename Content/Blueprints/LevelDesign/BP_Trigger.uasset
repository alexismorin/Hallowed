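; BP_Trigger is a level-design trigger that fires an empty TriggerEvent in response to the player or to damage.
; BP_Protag overlaps either register it as an interactable, cleared when the player leaves the Cube, or fire it immediately when Interactable is off.
; Interact, also called on any damage, shares the firing path, which a DoOnce flag can limit to a single activation.
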(event `self.ReceiveAnyDamage`
  (params (Damage :type "Float (single-precision)") (DamageType :type "DamageType Object Reference") (InstigatedBy :type "Controller Object Reference") (DamageCauser :type "Actor Object Reference"))
  (`self.Interact`))

(event `self.Cube.OnComponentEndOverlap`
  (params (OverlappedComponent :type "PrimitiveComponent Object Reference") (OtherActor :type "Actor Object Reference") (OtherComp :type "PrimitiveComponent Object Reference") (OtherBodyIndex :type Integer))
  (bind _asbp_protag (cast `/Game/Blueprints/BP_Protag` OtherActor))
  (if (`self.interactable`)
    (`/Game/Blueprints/BP_Protag.ExitInteractable` _asbp_protag)))

(event `self.ReceiveActorBeginOverlap`
  (params (OtherActor :type "Actor Object Reference"))
  (bind _asbp_protag (cast `/Game/Blueprints/BP_Protag` OtherActor))
  (set `self.player` _asbp_protag)
  (if (`self.interactable`)
    (`/Game/Blueprints/BP_Protag.EnterInteractable` (`self.player`) self)
    (else
      (if (`self.doOnce`) :!label _label
        (`/Engine/EditorBlueprintResources/StandardMacros.DoOnce` false
          (:`Completed`
            (`self.TriggerEvent`)))
        (else
          (`self.TriggerEvent`))))))

(event `TriggerEvent`)

(event `Interact`
  (goto _label))

(fn `UserConstructionScript`)